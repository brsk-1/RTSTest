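; RTS-style camera pawn that pans, zooms and rotates around a spring arm.
; WASD key events adjust two axis counters, which Tick feeds into movement input along the spring arm's forward and right vectors.
; Enhanced Input zoom changes the arm length within clamped limits.
; A trigger action toggles rotation mode, during which the rotate action yaws the spring arm.
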(event Input|EnhancedActionEvents|EnhancedInputActionIA_Zoom
  (params (ActionValue :type Float%20%28double-precision%29) (ElapsedSeconds :type Float%20%28double-precision%29) (TriggeredSeconds :type Float%20%28double-precision%29) (InputAction :type Input%20Action%20Object%20Reference :default "/Game/TopDown/Input/Actions/IA_Zoom.IA_Zoom"))
  (bind _springarm (Variables|Default|GetSpringArm))
  (:Triggered
    (Variables|/Script/Engine.SpringArmComponent|SetTargetArmLength _springarm (Math|Float|Clamp(Float) (+ (Variables|/Script/Engine.SpringArmComponent|GetTargetArmLength _springarm) (* ActionValue -1e+02)) 5e+02 1e+04))))

(event Input|EnhancedActionEvents|EnhancedInputActionIA_RotateTrigger
  (params (ActionValue :type Boolean) (ElapsedSeconds :type Float%20%28double-precision%29) (TriggeredSeconds :type Float%20%28double-precision%29) (InputAction :type Input%20Action%20Object%20Reference :default "/Game/TopDown/Input/Actions/IA_RotateTrigger.IA_RotateTrigger"))
  (:Triggered
    (if (Variables|Default|GetRotating)
      (Variables|Default|SetRotating false)
      (else
        (Variables|Default|SetRotating true)))))

(event Input|EnhancedActionEvents|EnhancedInputActionIA_Rotate
  (params (ActionValue :type Float%20%28double-precision%29) (ElapsedSeconds :type Float%20%28double-precision%29) (TriggeredSeconds :type Float%20%28double-precision%29) (InputAction :type Input%20Action%20Object%20Reference :default "/Game/TopDown/Input/Actions/IA_Rotate.IA_Rotate"))
  (bind _springarm (Variables|Default|GetSpringArm))
  (bind _returnvalue (Class|SpringArmComponent|GetTargetRotation _springarm))
  (:Triggered
    (if (Variables|Default|GetRotating)
      (Transformation|SetWorldRotation _springarm (Math|Rotator|MakeRotator (.roll _returnvalue) (.pitch _returnvalue) (+ (.yaw _returnvalue) (* ActionValue 1e+01))) false false))))

(event EventBeginPlay)

(event Collision|EventActorBeginOverlap
  (params (OtherActor :type Actor%20Object%20Reference)))

(event EventTick
  (params (DeltaSeconds :type Float%20%28single-precision%29))
  (bind _springarm (Variables|Default|GetSpringArm))
  (bind _springarm_2 (Variables|Default|GetSpringArm))
  (bind _returnvalue (Math|Vector|GetForwardVector _springarm))
  (bind _returnvalue_2 (Math|Vector|GetRightVector _springarm_2))
  (Pawn|Input|AddMovementInput (Math|Vector|MakeVector (.x _returnvalue) (.y _returnvalue) 0.0) (Variables|Default|GetUpDown) false)
  (Pawn|Input|AddMovementInput (Math|Vector|MakeVector (.x _returnvalue_2) (.y _returnvalue_2) 0.0) (Variables|Default|GetLeftRight) false))

(event Input|KeyboardEvents|W
  (params (Key :type Key%20Structure :default "None"))
  (bind _updown (Variables|Default|GetUpDown))
  (:Pressed
    (Math|Float|IncrementFloat _updown))
  (:Released
    (Math|Float|DecrementFloat _updown)))

(event Input|KeyboardEvents|A
  (params (Key :type Key%20Structure :default "None"))
  (bind _leftright (Variables|Default|GetLeftRight))
  (:Pressed
    (Math|Float|DecrementFloat _leftright))
  (:Released
    (Math|Float|IncrementFloat _leftright)))

(event Input|KeyboardEvents|S
  (params (Key :type Key%20Structure :default "None"))
  (bind _updown (Variables|Default|GetUpDown))
  (:Pressed
    (Math|Float|DecrementFloat _updown))
  (:Released
    (Math|Float|IncrementFloat _updown)))

(event Input|KeyboardEvents|D
  (params (Key :type Key%20Structure :default "None"))
  (bind _leftright (Variables|Default|GetLeftRight))
  (:Pressed
    (Math|Float|IncrementFloat _leftright))
  (:Released
    (Math|Float|DecrementFloat _leftright)))

(fn ConstructionScript)